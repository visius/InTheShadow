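; Game instance for the Shadow game that owns the save object reference and controls the main, level select and level menus.
; Save creates the ShadowSave slot if missing, then loads and caches it, without writing changes to an existing save.
; Show events lazily create and reuse widgets and enable the cursor, with both level menus removing the main menu.
; A quit event exits the game, while a UI-only input mode node is left unconnected.
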(event Custom|Show%20Main%20Menu
  (bind _returnvalue (Game|GetPlayerController 0))
  ;[1 1 1] Call Main Menu
  (Utilities|IsValid (Variables|Widget|GetMain%20Menu%20WB)
    (:Is%20Valid
      _)
    (:Is%20Not%20Valid
      (bind _returnvalue_2 (UserInterface|CreateWidget "/Game/Blueprints/Main_Menu.Main_Menu_C" _returnvalue))
      (bind _output_get (Variables|Widget|SetMain%20Menu%20WB _returnvalue_2))))
  (UserInterface|Viewport|AddtoViewport _output_get 0)
  (Variables|/Script/Engine.PlayerController|SetbShowMouseCursor _returnvalue true))

(event Custom|Show%20Level%20Select
  (bind _returnvalue (Game|GetPlayerController 0))
  ;[1 1 1] Cal level select menu
  (Utilities|IsValid (Variables|Widget|GetLevel%20Select%20WB)
    (:Is%20Valid
      _)
    (:Is%20Not%20Valid
      (bind _returnvalue_2 (UserInterface|CreateWidget "/Game/Blueprints/Level_Select.Level_Select_C" _returnvalue))
      (bind _output_get (Variables|Widget|SetLevel%20Select%20WB _returnvalue_2))))
  (UserInterface|Viewport|AddtoViewport _output_get 0)
  (Widget|RemovefromParent (Variables|Widget|GetMain%20Menu%20WB))
  (Variables|/Script/Engine.PlayerController|SetbShowMouseCursor _returnvalue true))

(event Custom|Save
  (bind _returnvalue (SaveGame|DoesSaveGameExist "ShadowSave_01"))
  (if _returnvalue
    _
    (else
      (bind _returnvalue_2 (SaveGame|CreateSaveGameObject "/Game/Blueprints/ShadowSave.ShadowSave_C"))
      (SaveGame|SaveGametoSlot _returnvalue_2 "ShadowSave_01")))
  (bind _returnvalue_3 (SaveGame|LoadGamefromSlot "ShadowSave_01"))
  (bind _asshadow_save (Utilities|Casting|CastToShadowSave _returnvalue_3))
  (Variables|Default|SetAs%20Shadow%20Save _asshadow_save))

(event Custom|Quit%20Game%20Event
  ;[1 1 1] Quit game
  (Game|QuitGame (Game|GetPlayerController 0) "Quit" false))

(event Custom|Show%20Level%20Menu
  (bind _returnvalue (Game|GetPlayerController 0))
  ;[1 1 1] Call level menu
  (Utilities|IsValid (Variables|Widget|GetLevel%20Menu%20WB)
    (:Is%20Valid
      _)
    (:Is%20Not%20Valid
      (bind _returnvalue_2 (UserInterface|CreateWidget "/Game/Blueprints/Level_menu.Level_menu_C" _returnvalue))
      (bind _output_get (Variables|Widget|SetLevel%20Menu%20WB _returnvalue_2))))
  (UserInterface|Viewport|AddtoViewport _output_get 0)
  (Variables|/Script/Engine.PlayerController|SetbShowMouseCursor _returnvalue true)
  (Widget|RemovefromParent (Variables|Widget|GetMain%20Menu%20WB)))