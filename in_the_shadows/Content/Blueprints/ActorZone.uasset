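; ActorZone is a puzzle target zone that detects when its MeshTarget is placed at the zone's position with near-zero rotation.
; Tick tests rotation and location against tolerance ranges, using timelines to lerp the mesh toward zero rotation and the zone's location.
; When both match, it locks once and increments BP_ShadowController's FinishCounter, copying it to the Shadow game instance.
; The construction script scales the Sphere by ZoneScale.
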(event EventBeginPlay
  (bind _outactors (Actor|GetAllActorsOfClass "/Game/Blueprints/BP_ShadowController.BP_ShadowController_C"))
  (Variables|Default|SetShadowController_ref (Utilities|Array|Get(acopy) _outactors))
  (Variables|Default|SetRotateComplete false)
  (Variables|Default|SetLocationComplete false)
  (Variables|Default|SetLockController false)
  (bind _asshadow_game_instance (Utilities|Casting|CastToShadow_GameInstance (Game|GetGameInstance)))
  (Variables|Default|SetShadow%20Game%20Instance%20ref _asshadow_game_instance))

(event Collision|EventActorBeginOverlap
  (params (OtherActor :type Actor%20Object%20Reference)))

(event EventTick
  (params (DeltaSeconds :type Float%20%28single-precision%29))
  (bind _returnvalue (Transformation|GetActorLocation))
  (bind _meshtarget (Variables|Default|GetMeshTarget))
  (bind _shadowcontroller_ref (Variables|Default|GetShadowController_ref))
  (bind _meshtarget_2 (Variables|Default|GetMeshTarget))
  (bind _rotaterange (Variables|Default|GetRotateRange))
  (bind _locationrange (Variables|Default|GetLocationRange))
  (bind _returnvalue_2 (Transformation|GetActorRotation _meshtarget_2))
  (bind _returnvalue_3 (Transformation|GetActorLocation _meshtarget))
  (bind _returnvalue_4 (+ _returnvalue _locationrange))
  (bind _returnvalue_5 (- _returnvalue _locationrange))
  (bind _returnvalue_6 (* _rotaterange -1.0))
  (if (not (Variables|Default|GetLockController))
    (if (Math|Boolean|ANDBoolean (Math|Float|InRange(Float) (.roll _returnvalue_2) _returnvalue_6 _rotaterange) (Math|Float|InRange(Float) (.pitch _returnvalue_2) _returnvalue_6 _rotaterange) (Math|Float|InRange(Float) (.yaw _returnvalue_2) _returnvalue_6 _rotaterange))
      (Variables|Default|SetRotateComplete true)
      (Timeline|Timeline_2 Play
        (:Update
          (CallFunction|FinalazeRotation)))
      (else
        (Variables|Default|SetRotateComplete false)))
    (if (Math|Boolean|ANDBoolean (Math|Float|InRange(Float) (.x _returnvalue_3) (.x _returnvalue_5) (.x _returnvalue_4)) (Math|Float|InRange(Float) (.y _returnvalue_3) (.y _returnvalue_5) (.y _returnvalue_4)) (Math|Float|InRange(Float) (.z _returnvalue_3) (.z _returnvalue_5) (.z _returnvalue_4)))
      (Variables|Default|SetLocationComplete true)
      (Timeline|Timeline_1 Play
        (:Update
          (CallFunction|FinalazeLocation)
          (if (and (Variables|Default|GetRotateComplete) (Variables|Default|GetLocationComplete))
            (Utilities|FlowControl|DoOnce false
              (:Completed
                (Variables|Default|SetLockController true)
                (bind _output_get (Variables|/Game/Blueprints/BP_ShadowController.BP_ShadowController_C|SetFinishCounter _shadowcontroller_ref (+ (Variables|/Game/Blueprints/BP_ShadowController.BP_ShadowController_C|GetFinishCounter _shadowcontroller_ref) 1)))
                (Variables|/Game/Blueprints/Shadow_GameInstance.Shadow_GameInstance_C|SetFinishCounter (Variables|Default|GetShadow%20Game%20Instance%20ref) _output_get))))))
      (else
        (Variables|Default|SetLocationComplete false)))))

(fn ConstructionScript
  (bind _meshtarget (Variables|Default|GetMeshTarget))
  (AddComponent|AddStaticMeshComponent _meshtarget false (Transformation|GetActorTransform _meshtarget))
  (Transformation|SetRelativeScale3D (Variables|Default|GetSphere) (* "1.000000,1.000000,1.000000" (Variables|Default|GetZoneScale))))

(fn FinalazeLocation
  (Transformation|SetActorLocation (Variables|Default|GetMeshTarget) (Math|Vector|Lerp(Vector) (Transformation|GetActorLocation (Variables|Default|GetMeshTarget)) (Transformation|GetActorLocation) 0.1) false false)
  (return))

(fn FinalazeRotation
  (bind _meshtarget (Variables|Default|GetMeshTarget))
  (Transformation|SetActorRotation _meshtarget (Math|Rotator|Lerp(Rotator) (Transformation|GetActorRotation _meshtarget) "0, 0, 0" 0.1))
  (return))