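; Player controller actor for a shadow puzzle level that manipulates ActorZone target meshes and handles level completion.
; Mouse wheel cycles through the zones found at BeginPlay.
; Holding left or right mouse opens Tick-driven gates that rotate or move the selected mesh, unless LockController is set.
; Tick compares externally updated FinishCounter to zone count, then repeatedly fires the completion menu event and, outside test mode, saves current and next level states.
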(event EventBeginPlay
  (Variables|Default|SetFinishCounter 0)
  (Variables|Default|SetItemSelector 0)
  (Input|EnableInput (Game|GetPlayerController 0))
  (bind _outactors (Actor|GetAllActorsOfClass "/Game/Blueprints/ActorZone.ActorZone_C"))
  (bind _output_get (Variables|Default|SetOut%20Actors _outactors))
  (bind _output_get_2 (Variables|Default|SetActor%20Target (Utilities|Array|Get(acopy) _output_get (Variables|Default|GetItemSelector))))
  (Variables|Default|SetMesh%20Target (Variables|/Game/Blueprints/ActorZone.ActorZone_C|GetMeshTarget _output_get_2))
  (bind _asshadow_game_instance (Utilities|Casting|CastToShadow_GameInstance (Game|GetGameInstance)))
  (Variables|Default|SetGameInstance_ref _asshadow_game_instance))

(event Collision|EventActorBeginOverlap
  (params (OtherActor :type Actor%20Object%20Reference)))

(event EventTick
  (params (DeltaSeconds :type Float%20%28single-precision%29))
  (bind _gameinstance_ref (Variables|Default|GetGameInstance_ref))
  (bind _gameinstance_ref_2 (Variables|Default|GetGameInstance_ref))
  (bind _gameinstance_ref_3 (Variables|Default|GetGameInstance_ref))
  (bind _as_shadow_save (Variables|/Game/Blueprints/Shadow_GameInstance.Shadow_GameInstance_C|GetAs%20Shadow%20Save _gameinstance_ref))
  (bind _level_id (Variables|/Game/Blueprints/Shadow_GameInstance.Shadow_GameInstance_C|GetLevel_ID _gameinstance_ref_3))
  (bind _levelstate_01 (Variables|/Game/Blueprints/ShadowSave.ShadowSave_C|GetLevelState_01 _as_shadow_save))
  (Utilities|FlowControl|Sequence
    (:then_0
      ;[1 1 1] Rotate Actors
      (Utilities|FlowControl|Gate true
        (:Exit
          (Class|Actor|AddActorWorldRotation (Variables|Default|GetMesh%20Target) (Math|Rotator|MakeRotator 0.0 (* (Variables|Default|GetrotateY) (* (Class|Actor|GetInputAxisKeyValue) -1.0)) (* (Class|Actor|GetInputAxisKeyValue) -1.0))))))
    (:then_1
      ;[1 1 1] Move Actors
      (Utilities|FlowControl|Gate true
        (:Exit
          (Transformation|AddActorWorldOffset (Variables|Default|GetMesh%20Target) (Math|Vector|MakeVector 0.0 (Class|Actor|GetInputAxisKeyValue) (Class|Actor|GetInputAxisKeyValue))))))
    (:then_2
      (Variables|Default|SetLevelComplete (== (Variables|Default|GetFinishCounter) (Utilities|Array|Length (Variables|Default|GetOut%20Actors))))
      (if (Variables|Default|GetLevelComplete)
        (Default|EventLevelComplete (Variables|/Game/Blueprints/Shadow_GameInstance.Shadow_GameInstance_C|GetLevel%20Menu%20WB (Variables|Default|GetGameInstance_ref)))
        (if (not (Variables|/Game/Blueprints/Shadow_GameInstance.Shadow_GameInstance_C|GetIs%20Test%20Menu (Variables|Default|GetGameInstance_ref)))
          (Utilities|Array|SetArrayElem (Variables|/Game/Blueprints/ShadowSave.ShadowSave_C|GetLevelState_01 (Variables|/Game/Blueprints/Shadow_GameInstance.Shadow_GameInstance_C|GetAs%20Shadow%20Save _gameinstance_ref_2)) (- (Variables|/Game/Blueprints/Shadow_GameInstance.Shadow_GameInstance_C|GetLevel_ID _gameinstance_ref_2) 1) 2)
          (if (> _level_id (Utilities|Array|LastIndex _levelstate_01))
            _
            (else
              (Utilities|Array|SetArrayElem _levelstate_01 _level_id 1)))
          (SaveGame|SaveGametoSlot (Variables|/Game/Blueprints/Shadow_GameInstance.Shadow_GameInstance_C|GetAs%20Shadow%20Save (Variables|Default|GetGameInstance_ref)) "ShadowSave_01"))))))

(event Input|MouseEvents|MouseWheelAxis
  (params (AxisValue :type Float%20%28single-precision%29))
  ;[1 1 1] Select actors
  (if (< AxisValue 0.0)
    (bind _output_get (Variables|Default|SetItemSelector (- (Variables|Default|GetItemSelector) 1)))
    (if (< _output_get 0)
      (Variables|Default|SetItemSelector (Utilities|Array|LastIndex (Variables|Default|GetOut%20Actors))))
    (bind _output_get_2 (Variables|Default|SetActor%20Target (Utilities|Array|Get(acopy) (Variables|Default|GetOut%20Actors) (Variables|Default|GetItemSelector)) :!label _label))
    (Variables|Default|SetMesh%20Target (Variables|/Game/Blueprints/ActorZone.ActorZone_C|GetMeshTarget _output_get_2))
    (Development|PrintString (Utilities|GetDisplayName (Utilities|Array|Get(acopy) (Variables|Default|GetOut%20Actors) (Variables|Default|GetItemSelector))))
    (elif (> AxisValue 0.0)
      (bind _output_get_3 (Variables|Default|SetItemSelector (+ (Variables|Default|GetItemSelector) 1)))
      (if (> _output_get_3 (Utilities|Array|LastIndex (Variables|Default|GetOut%20Actors)))
        (Variables|Default|SetItemSelector 0)
        (goto _label)
        (else
          (goto _label))))))

(event Input|KeyboardEvents|0
  (params (Key :type Key%20Structure :default "None")))

(event Input|MouseEvents|RightMouseButton
  (params (Key :type Key%20Structure :default "None"))
  ;[1 1 1] Move Actors
  (:Pressed
    (if (Variables|/Game/Blueprints/ActorZone.ActorZone_C|GetLockController (Variables|Default|GetActor%20Target))
      (Utilities|FlowControl|Gate true) ; enters at Close
      (else
        (Utilities|FlowControl|Gate true) ; enters at Open
      )))
  (:Released
    (Utilities|FlowControl|Gate true) ; enters at Close
  ))

(event Input|MouseEvents|LeftMouseButton
  (params (Key :type Key%20Structure :default "None"))
  ;[1 1 1] Rotate Actors
  (:Pressed
    (if (Variables|/Game/Blueprints/ActorZone.ActorZone_C|GetLockController (Variables|Default|GetActor%20Target))
      (Utilities|FlowControl|Gate true) ; enters at Close
      (else
        (Utilities|FlowControl|Gate true) ; enters at Open
      )))
  (:Released
    (Utilities|FlowControl|Gate true) ; enters at Close
  ))

(event Input|KeyboardEvents|LeftShift
  (params (Key :type Key%20Structure :default "None")))

(event Input|MouseEvents|MouseWheelDown
  (params (Key :type Key%20Structure :default "None")))

(event Input|MouseEvents|MouseWheelUp
  (params (Key :type Key%20Structure :default "None")))

(fn ConstructionScript
  (Transformation|SetActorLocation "0,0.000000,20.000000" false false))